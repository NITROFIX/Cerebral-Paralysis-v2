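; Parent Blueprint for candle cluster props that can be set as burning or off through CandleBurnType.
; The construction script swaps the material on meshes tagged Candle and toggles particle systems tagged CandleFire to match that state.
; In the Off state it also zeroes and hides every spot light component, with no branch that sets light values for Burning.
; The event graph has no active logic.
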(fn `UserConstructionScript`
  (`SceneComponent.SetVisibility` (`self.DefaultSceneRoot`) true true)
  (for _array_element (`self.GetComponentsByTag` "/Script/Engine.StaticMeshComponent" "Candle")
    (`PrimitiveComponent.SetMaterial` _array_element 0 (select `/Game/1_Plugins/Bazaar_Meshingun/Blueprint/Candle/E_CandleBurnType` (`self.candleBurnType`) :`NewEnumerator0` "/Game/1_Plugins/Bazaar_Meshingun/Blueprint/Candle/MI_Candle_Burning_01a.MI_Candle_Burning_01a" :`NewEnumerator2` "/Game/1_Plugins/Bazaar_Meshingun/Blueprint/Candle/MI_Candle_Off_01a.MI_Candle_Off_01a" :!type "MaterialInterface Object Reference")))
  (for _array_element_2 (`self.GetComponentsByTag` "/Script/Engine.ParticleSystemComponent" "CandleFire")
    (`SceneComponent.SetVisibility` _array_element_2 (select `/Game/1_Plugins/Bazaar_Meshingun/Blueprint/Candle/E_CandleBurnType` (`self.candleBurnType`) :`NewEnumerator0` true) true))
  (for _array_element_3 (`self.K2_GetComponentsByClass` "/Script/Engine.SpotLightComponent")
    (if (`|EnumEquality` (`self.candleBurnType`) "NewEnumerator2")
      (`LightComponent.SetIntensity` _array_element_3 0.0)
      (`SceneComponent.SetVisibility` _array_element_3 false false)
      (`SceneComponent.SetHiddenInGame` _array_element_3 true true))))