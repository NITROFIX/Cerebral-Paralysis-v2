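; Enemy shotgun bullet that damages whatever it hits through that actor's HealthComponent.
; A sphere overlap checks CanTakeDamage against the bullet's team, applies fixed damage, then detaches the trail VFX and destroys the bullet.
; Actors without a HealthComponent also destroy it, while those that refuse damage leave it alive.
; On destruction, the VFXTrailPlayer is told to destroy its trail actor.
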(event `self.ReceiveBeginPlay`
  (add `PrimitiveComponent.OnComponentBeginOverlap` (`self.Sphere`) (delegate `OnOverlap`)))

(event `OnOverlap`
  (params (OverlappedComponent :type "PrimitiveComponent Object Reference") (OtherActor :type "Actor Object Reference") (OtherComp :type "PrimitiveComponent Object Reference") (OtherBodyIndex :type Integer) (bFromSweep :type Boolean) (SweepResult :type "HitResult Structure (by ref)"))
  (bind _returnvalue (`self.GetComponentByClass` OtherActor "/Script/CerebralParalysis_v2.HealthComponent"))
  (bind _returnvalue_2 (`self.GetTeam`))
  (`/Engine/EditorBlueprintResources/StandardMacros.IsValid` OtherActor
    (:`Is Valid`
      (`/Engine/EditorBlueprintResources/StandardMacros.IsValid` _returnvalue
        (:`Is Valid`
          (bind _returnvalue_3 (`HealthComponent.CanTakeDamage` _returnvalue _returnvalue_2))
          (if _returnvalue_3
            (`HealthComponent.TakeDamage` _returnvalue _returnvalue_2 10.0)
            (`VFXTrailPlayer.DetachSystem` (`self.VFXTrailPlayer`) :!label _label)
            (`self.K2_DestroyActor`)))
        (:`Is Not Valid`
          (goto _label))))))

(event `self.ReceiveDestroyed`
  (`VFXTrailPlayer.DestroyTrailActor` (`self.VFXTrailPlayer`)))

(fn `UserConstructionScript`)