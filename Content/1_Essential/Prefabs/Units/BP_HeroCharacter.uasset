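; Hero character Blueprint that provides smoothed movement speed and running direction; its event graph and construction script are empty.
; GetRunningAngle derives a signed angle between actor forward and velocity, using the dot product for magnitude and cross product Z for side.
; GetSpeed takes the velocity's length.
; Both lerp a stored previous value by DeltaTime times ChangeSpeed, and their returns apply that lerp again to the updated value.
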(fn `GetRunningAngle`
  (params (DeltaTime :type "Float (double-precision)"))
  (returns (Angle :type "Float (double-precision)"))
  (bind _returnvalue (`self.GetActorForwardVector`))
  (bind _returnvalue_2 (`KismetMathLibrary.Normal` (`MovementComponent.Velocity` (`self.CharacterMovement`))))
  (bind (_returnvalue_x _returnvalue_y _returnvalue_z) (`KismetMathLibrary.BreakVector` (`KismetMathLibrary.Cross_VectorVector` _returnvalue _returnvalue_2)))
  (bind _returnvalue_3 (`KismetMathLibrary.Lerp` (`self.OldRotation`) (* (`KismetMathLibrary.DegAcos` (`KismetMathLibrary.Dot_VectorVector` _returnvalue _returnvalue_2)) (`KismetMathLibrary.SignOfFloat` _returnvalue_z)) (* DeltaTime (`self.ChangeSpeed`))))
  (set `self.OldRotation` _returnvalue_3)
  (return _returnvalue_3))

(fn `GetSpeed`
  (params (DeltaTime :type "Float (double-precision)"))
  (returns (Velocity :type "Float (double-precision)"))
  (bind _returnvalue (`KismetMathLibrary.Lerp` (`self.OldVelocity`) (`KismetMathLibrary.Vector_Distance` (`MovementComponent.Velocity` (`self.CharacterMovement`))) (* DeltaTime (`self.ChangeSpeed`))))
  (set `self.OldVelocity` _returnvalue)
  (return _returnvalue))

(fn `UserConstructionScript`)