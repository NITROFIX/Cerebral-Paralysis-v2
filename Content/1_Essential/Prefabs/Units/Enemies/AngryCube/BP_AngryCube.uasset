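; BP_AngryCube is an enemy unit that shoots at the player in time with the music.
; On BeginPlay it binds to the music sequencer subsystem's easy-hit event, and each hit forces its BasicWeapon to fire.
; Every tick it turns toward the player from the player provider subsystem with pitch zeroed, and sets the weapon direction the same way, keeping its aim horizontal.
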(event `self.ReceiveBeginPlay`
  (add `MusicSequencerSubsystem.OnEasyHit` (subsystem `MusicSequencerSubsystem`) (delegate `OnEasyHit`)))

(event `OnEasyHit`
  (`BasicWeaponComponent.ForceFire` (`self.BasicWeapon`)))

(event `self.ReceiveTick`
  (params (DeltaSeconds :type "Float (single-precision)"))
  (bind _returnvalue (`KismetMathLibrary.MakeRotator` (.roll (`KismetMathLibrary.FindLookAtRotation` (`self.K2_GetActorLocation`) (`self.K2_GetActorLocation` (`PlayerProviderSubsystem.GetPlayer` (subsystem `PlayerProviderSubsystem`))))) 0.0 (.yaw (`KismetMathLibrary.FindLookAtRotation` (`self.K2_GetActorLocation`) (`self.K2_GetActorLocation` (`PlayerProviderSubsystem.GetPlayer` (subsystem `PlayerProviderSubsystem`)))))))
  (`self.K2_SetActorRotation` _returnvalue)
  (`BasicWeaponComponent.SetDirection` (`self.BasicWeapon`) _returnvalue))

(fn `UserConstructionScript`)