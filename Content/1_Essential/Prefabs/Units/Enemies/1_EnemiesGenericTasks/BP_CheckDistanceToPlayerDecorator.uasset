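; Behavior tree decorator for enemy AI that gates a branch on the controlled pawn's distance to the player.
; It reads the player actor from the PlayerObject blackboard key and fails if that is not a valid Actor.
; ActionType selects the comparison, with Distance as the left operand, so "<" passes when the player is farther away than Distance.
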(fn `PerformConditionCheckAI`
  (params (OwnerController :type "AIController Object Reference") (ControlledPawn :type "Pawn Object Reference"))
  (returns (ReturnValue :type Boolean))
  (bind _distance (`self.Distance`))
  (bind _asactor (cast `Actor` (`BTFunctionLibrary.GetBlackboardValueAsObject` (`self.PlayerObject`)))
    (:`then`
      (switch `ECompareOperationEnum` (`self.ActionType`)
        (:`Dataflow_Compare_Equal`
          (bind _returnvalue (`KismetMathLibrary.VSize` (- (`Actor.K2_GetActorLocation` _asactor) (`Actor.K2_GetActorLocation` ControlledPawn))))
          (if (== _distance _returnvalue)
            _
            (else
              (return false))))
        (:`Dataflow_Compare_Smaller`
          (if (< _distance _returnvalue)
            _
            (else
              (return false))))
        (:`Dataflow_Compare_SmallerOrEqual`
          (if (<= _distance _returnvalue)
            _
            (else
              (return false))))
        (:`Dataflow_Compare_Greater`
          (if (> _distance _returnvalue)
            _
            (else
              (return false))))
        (:`Dataflow_Compare_GreaterOrEqual`
          (if (>= _distance _returnvalue)
            _
            (else
              (return false)))))
      (return true))
    (:`CastFailed`
      (return false))))