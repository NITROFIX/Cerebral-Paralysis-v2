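; Behavior Tree task for enemy AI that picks a point away from the player and writes it to the move-target Blackboard key.
; It offsets the pawn's location along the direction away from the player actor, scaled by away distance, scare amount and inverse separation, so closer players push it farther.
; It prints the offset length for debugging, then finishes successfully, or aborts when no player actor is found.
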(event `self.ReceiveExecuteAI`
  (params (OwnerController :type "AIController Object Reference") (ControlledPawn :type "Pawn Object Reference"))
  (bind _returnvalue (`Actor.K2_GetActorLocation` ControlledPawn))
  (bind _asactor (cast `Actor` (`BTFunctionLibrary.GetBlackboardValueAsObject` (`self.PlayerValue`)))
    (:`then`
      (bind _returnvalue_2 (- _returnvalue (`Actor.K2_GetActorLocation` _asactor)))
      (bind _returnvalue_3 (* (* (`KismetMathLibrary.Normal` _returnvalue_2) (`self.AwayDistance`)) (* (/ (`self.InversingPower`) (`KismetMathLibrary.VSize` _returnvalue_2)) (`self.ScareAmount`))))
      (`BTFunctionLibrary.SetBlackboardValueAsVector` (`self.MoveTargetValue`) (+ _returnvalue _returnvalue_3))
      (`KismetSystemLibrary.PrintString` (`KismetStringLibrary.Conv_DoubleToString` (`KismetMathLibrary.VSize` _returnvalue_3)))
      (`self.FinishExecute` true))
    (:`CastFailed`
      (`self.FinishAbort`))))