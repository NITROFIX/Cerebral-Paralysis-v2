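; BP_Ancient is an enemy unit that faces the player and fires its weapon in time with the music.
; On BeginPlay it binds to the MusicSequencerSubsystem's easy and medium hit events, each firing AIWeapon at the matching difficulty.
; Every tick it rotates toward the player with pitch locked at zero and passes the player's location to AIWeapon as the aim point.
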(event `self.ReceiveBeginPlay`
  (add `MusicSequencerSubsystem.OnEasyHit` (subsystem `MusicSequencerSubsystem`) (delegate `OnEasyHit`))
  (add `MusicSequencerSubsystem.OnMediumHit` (subsystem `MusicSequencerSubsystem`) (delegate `OnMediumHit`)))

(event `OnEasyHit`
  (`AIWeaponComponent.Fire` (`self.AIWeapon`) "Easy"))

(event `OnMediumHit`
  (`AIWeaponComponent.Fire` (`self.AIWeapon`) "Medium"))

(event `self.ReceiveTick`
  (params (DeltaSeconds :type "Float (single-precision)"))
  (bind _returnvalue (`self.K2_GetActorLocation` (`PlayerProviderSubsystem.GetPlayer` (subsystem `PlayerProviderSubsystem`))))
  (`self.K2_SetActorRotation` (`KismetMathLibrary.MakeRotator` (.roll (`KismetMathLibrary.FindLookAtRotation` (`self.K2_GetActorLocation`) _returnvalue)) 0.0 (.yaw (`KismetMathLibrary.FindLookAtRotation` (`self.K2_GetActorLocation`) _returnvalue))))
  (`BasicWeaponComponent.SetAimLocation` (`self.AIWeapon`) _returnvalue))

(fn `UserConstructionScript`)