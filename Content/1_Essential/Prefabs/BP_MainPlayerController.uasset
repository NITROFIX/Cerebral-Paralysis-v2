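; BP_MainPlayerController is a player controller that switches between the regular pawn and a free spectator pawn with number keys.
; Key 1 possesses the stored spectator, or on first use caches the current pawn and spawns a SpectatorPawn at its transform.
; Key 2 repossesses the cached regular pawn if it is valid.
; The spectator is reused, so later switches return to wherever it was left.
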(event `Key|One`
  (params (Key :type "Key Structure"))
  (bind _returnvalue (`GameplayStatics.GetPlayerPawn` 0))
  (:`Pressed`
    (if (`KismetSystemLibrary.IsValid` (`self.SpecPawn`))
      (`self.Possess` (`self.SpecPawn`))
      (else
        (set `self.RegularPawn` _returnvalue)
        (bind _returnvalue_2 (`|SpawnActorFromClass` "/Script/Engine.SpectatorPawn" (`self.GetTransform` _returnvalue) "Undefined" "MultiplyWithRoot" null null))
        (`self.Possess` _returnvalue_2)
        (set `self.SpecPawn` _returnvalue_2)))))

(event `Key|Two`
  (params (Key :type "Key Structure"))
  (:`Pressed`
    (if (`KismetSystemLibrary.IsValid` (`self.RegularPawn`))
      (`self.Possess` (`self.RegularPawn`)))))

(fn `UserConstructionScript`)