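; Spawner that scatters a small random number of area effects around the player and later detonates them together.
; Spawn line-traces toward the ground from random offsets within AreasSpawnDistance of the player, then spawns an AreaEffect actor and passes it the hit location and a random radius.
; Explode triggers every tracked effect and clears the list; NewFunction is an empty stub.
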(fn `Explode`
  (bind _spawnedactors (`self.SpawnedActors`))
  (for _array_element _spawnedactors
    (`/Game/1_Essential/Prefabs/Spawners/BP_AreaEffectActor.Explode` _array_element))
  (`KismetArrayLibrary.Array_Clear` _spawnedactors))

(fn `NewFunction`
  (params (NewParam :type Integer)))

(fn `Spawn`
  (bind _areasspawndistance (`self.AreasSpawnDistance`))
  (bind _returnvalue (+ (`KismetMathLibrary.MakeVector` (* (`KismetMathLibrary.RandomFloatInRange` -1.0 1.0) _areasspawndistance) (* (`KismetMathLibrary.RandomFloatInRange` -1.0 1.0) _areasspawndistance)) (`self.K2_GetActorLocation` (`PlayerProviderSubsystem.GetPlayer` (subsystem `PlayerProviderSubsystem`)))))
  (for _ (range (+ (`KismetMathLibrary.Conv_Int64ToInt` (`KismetMathLibrary.RandomInteger64InRange` 2 5)) 1))
    (bind _outhit (`KismetSystemLibrary.LineTraceSingle` _returnvalue (`KismetMathLibrary.MakeVector` (.x _returnvalue) (.y _returnvalue) -100.0) "TraceTypeQuery1"))
    (bind _returnvalue_2 (`|SpawnActorFromClass` (`self.AreaEffect`) (`self.GetLevelTransform`) "AlwaysSpawn" "MultiplyWithRoot" null null))
    (`/Game/1_Essential/Prefabs/Spawners/BP_AreaEffectActor.Spawn` _returnvalue_2 (`KismetMathLibrary.RandomFloatInRange` 2.0 5.0) (`.Location` (`GameplayStatics.BreakHitResult` _outhit)))
    (`KismetArrayLibrary.Array_Add` (`self.SpawnedActors`) _returnvalue_2)))

(fn `UserConstructionScript`)