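; BP_AreaEffectActor is an actor that shows the visuals for a circular area effect, from its spawn marker to its explosion.
; Spawn stores the radius and a slightly raised position, then starts a Niagara system with scale and ring parameters derived from the radius.
; Explode deactivates that system and plays an explosion system at the stored position, sized from the same radius.
; The graphs handle visuals only, with no damage or timing logic.
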(fn `Explode`
  (`ActorComponent.Deactivate` (`self.Spawn System Instance`))
  (bind _returnvalue (`NiagaraFunctionLibrary.SpawnSystemAtLocation` (`self.Explosion Niagara System`) (`self.SpawnPosition`)))
  (`NiagaraComponent.SetVariableFloat` _returnvalue (`self.ExplosionSizeParameterName`) (* (`self.Radius`) 0.2)))

(fn `Spawn`
  (params (Radius :type "Float (double-precision)") (Location :type "Vector Structure"))
  (bind _returnvalue (+ Location (0.0 0.0 0.1)))
  (bind _output_get (set `self.Radius` Radius))
  (set `self.SpawnPosition` _returnvalue)
  (bind _returnvalue_2 (`NiagaraFunctionLibrary.SpawnSystemAtLocation` (`self.Spawn Niagara System`) _returnvalue))
  (bind _output_get_2 (set `self.Spawn System Instance` _returnvalue_2))
  (`NiagaraComponent.SetVariableFloat` _output_get_2 (`self.ScaleParameterName`) _output_get)
  (`NiagaraComponent.SetVariableFloat` _returnvalue_2 (`self.RingParameterName`) (* _output_get 15.0)))

(fn `UserConstructionScript`)